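; BP_ModKillVolume is a mod-facing placeholder actor that stands in for the game's BP_KillVolume.
; Its construction script sizes a Box component from an Extent variable.
; On BeginPlay it spawns a BP_KillVolume at its own transform, owned by itself, and copies the box extent onto the spawned volume's BoxComponent.
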(event EventBeginPlay
  (bind _returnvalue (Game|SpawnActorfromClass "/Game/Environment/FieldGimmick/Blueprints/BP_KillVolume.BP_KillVolume_C" (Transformation|GetActorTransform) "AlwaysSpawn" self 0))
  (Components|Box|SetBoxExtent (Actor|GetComponentbyClass _returnvalue "/Script/Engine.BoxComponent") (Variables|/Script/Engine.BoxComponent|GetBoxExtent (Variables|Default|GetBox)) true))

(fn ConstructionScript
  (Components|Box|SetBoxExtent (Variables|Default|GetBox) (Variables|Volume|GetExtent) true))