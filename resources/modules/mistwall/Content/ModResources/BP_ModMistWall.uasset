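; BP_ModMistWall is a mod-resource stand-in for a mist wall, spawning the real BP_MistWall at its transform on BeginPlay with its width, height and initial state.
; The construction script scales and positions a collision box and an editor placeholder mesh from Width and Height.
; SetState forwards enable and force to the spawned wall and, when EmulateCollision is set, switches the box between boss-wall and no-collision profiles.
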(event EventBeginPlay
  (bind _returnvalue (Game|SpawnActorfromClass "/Game/User/Shift_Tadokoro/MistWall/BP_MistWall.BP_MistWall_C" (Transformation|GetActorTransform) "AlwaysSpawn" self (Variables|MistWall|GetInitial%20Enable) (Variables|MistWall|GetWidth) (Variables|MistWall|GetHeight) 0))
  (Variables|Default|SetMistWall _returnvalue))

(fn ConstructionScript
  (bind _collision (Variables|Default|GetCollision))
  (bind _placeholdermesh (Variables|Default|GetPlaceholderMesh))
  (Utilities|FlowControl|Sequence
    (:then_0
      (LocalVariables|SetActualWidth (* (Variables|MistWall|GetWidth) 5.2))
      (LocalVariables|SetActualHeight (* (Variables|MistWall|GetHeight) 3.5)))
    (:then_1
      ;[1 1 1] Collision
      (Components|Box|SetBoxExtent _collision (Math|Vector|MakeVector (* (LocalVariables|GetActualWidth) 5e+01) 2.0 (* (LocalVariables|GetActualHeight) 5e+01)) true)
      (Transformation|SetRelativeLocation _collision (Math|Vector|MakeVector 0.0 0.0 (* (LocalVariables|GetActualHeight) 5e+01)) false true)
      (if (Variables|MistWall|GetEmulate%20Collision)
        (CallFunction|SetCollision (Variables|MistWall|GetInitial%20Enable))
        (else
          (CallFunction|SetCollision false))))
    (:then_2
      ;[1 1 1] In Editor Placeholder Mesh
      (Utilities|IsValid _placeholdermesh
        (:Is%20Valid
          (Transformation|SetRelativeScale3D _placeholdermesh (Math|Vector|MakeVector (LocalVariables|GetActualWidth) 0.1 (LocalVariables|GetActualHeight)))
          (Transformation|SetRelativeLocation _placeholdermesh (Math|Vector|MakeVector 0.0 0.0 (* (LocalVariables|GetActualHeight) 5e+01)) false false))))))

(fn SetState
  (params (Enable :type Boolean) (Force :type Boolean))
  (Default|SetStateMistWall (Variables|Default|GetMistWall) Enable Force)
  (if (Variables|MistWall|GetEmulate%20Collision)
    (CallFunction|SetCollision Enable)))

(fn SetCollision
  (params (Enable :type Boolean))
  (bind _collision (Variables|Default|GetCollision))
  (if Enable
    (Collision|SetCollisionProfileName _collision "GEZ_BossWallAfter" :!class /Script/Engine.PrimitiveComponent)
    (else
      (Collision|SetCollisionProfileName _collision "NoCollision" :!class /Script/Engine.PrimitiveComponent))))