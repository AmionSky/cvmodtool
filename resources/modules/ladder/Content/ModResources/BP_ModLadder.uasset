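; BP_ModLadder is an adjustable-height ladder for mods that wraps the game's BP_Ladder.
; The construction script optionally snaps Height to a 50-unit grid, then places top and bottom meshes and stacks loop segments between them.
; On BeginPlay it spawns a BP_Ladder and finds its components by object name.
; It then moves the top climb areas and locator, stretches the middle binding box to fit, and clears the default meshes.
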(event EventBeginPlay
  (bind _returnvalue (Transformation|GetActorTransform))
  (bind _returnvalue_2 (Game|SpawnActorfromClass "/Game/Environment/FieldGimmick/Blueprints/BP_Ladder.BP_Ladder_C" (Math|Transform|MakeTransform (Math|Vector|MakeVector (.x (.location _returnvalue)) (.y (.location _returnvalue)) (- (.z (.location _returnvalue)) (Variables|Ladder|GetModelOffset))) (.rotation _returnvalue) (.scale _returnvalue)) "AlwaysSpawn" self 0))
  (Variables|Default|SetLadder _returnvalue_2)
  (CallFunction|QueryComponents)
  (CallFunction|SetupTop)
  (CallFunction|SetupMiddle)
  ;[1 1 1] Disable default mesh
  (Components|StaticMesh|SetStaticMesh (Variables|Default|GetTopMesh) 0)
  (Components|StaticMesh|SetStaticMesh (Variables|Default|GetBottomMesh) 0))

(fn ConstructionScript
  (bind _laddertop (Variables|Default|GetLadderTop))
  (bind _height (Variables|Ladder|GetHeight))
  (bind (_remainder _returnvalue) (Math|Float|Division(WholeandRemainder) _height 2e+02))
  (bind _relativelocation (Variables|/Script/Engine.SceneComponent|GetRelativeLocation _laddertop))
  (CallFunction|AdjustHeight)
  ;[1 1 1] Set Meshes
  (Components|StaticMesh|SetStaticMesh (Variables|Default|GetLadderTop) (Variables|Ladder|GetMeshTop))
  (Components|StaticMesh|SetStaticMesh (Variables|Default|GetLadderBottom) (Variables|Ladder|GetMeshBottom))
  ;[1 1 1] Top
  (Transformation|SetRelativeLocation (Variables|Default|GetArrowTop) (Math|Vector|MakeVector 0.0 0.0 (+ (Variables|Ladder|GetHeight) 5e+01)) false false)
  (Transformation|SetRelativeLocation _laddertop (Math|Vector|MakeVector (.x _relativelocation) (.y _relativelocation) (- (Utilities|GetHeightValue) 11.347717)) false false)
  ;[1 1 1] Ladder Loop
  (for _index (range 0 (- _returnvalue 1))
    (bind _returnvalue_2 (AddComponent|AddStaticMeshComponent false (Math|Transform|MakeTransform (Math|Vector|MakeVector 0.0 (LocalVariables|GetLoopYOffset) (- (Utilities|LoopOffset (Variables|Ladder|GetHeight)) (* _index 2e+02))) "0, 0, 0" "1,1,1")))
    (Components|StaticMesh|SetStaticMesh _returnvalue_2 (Variables|Ladder|GetMeshLoop)))
  (if (> _remainder 1e+01)
    (bind _returnvalue_3 (AddComponent|AddStaticMeshComponent false (Math|Transform|MakeTransform (Math|Vector|MakeVector 0.0 (LocalVariables|GetLoopYOffset) (Utilities|LoopOffset _remainder)) "0, 0, 0" "1,1,1")))
    (Components|StaticMesh|SetStaticMesh _returnvalue_3 (Variables|Ladder|GetMeshLoop))))

(fn SetupTop
  (bind _bindingareatop (Variables|Default|GetBindingAreaTop))
  (bind _bindingareatop_2 (Variables|Default|GetBindingAreaTop))
  (bind _relativelocation (Variables|/Script/Engine.SceneComponent|GetRelativeLocation _bindingareatop_2))
  (bind _relativelocation_2 (Variables|/Script/Engine.SceneComponent|GetRelativeLocation _bindingareatop))
  ;[1 1 1] Calculate Bind Location
  (LocalVariables|SetBindTarget (Math|Vector|MakeVector (.x _relativelocation_2) (.y _relativelocation_2) (Utilities|GetHeightValue)))
  ;[1 1 1] Calculate End and Locator Location
  (LocalVariables|SetEndTarget (+ (- (Variables|/Script/Engine.SceneComponent|GetRelativeLocation (Variables|Default|GetEndAreaClimbUp)) _relativelocation) (LocalVariables|GetBindTarget)))
  (LocalVariables|SetLocTarget (+ (LocalVariables|GetBindTarget) (- (Variables|/Script/Engine.SceneComponent|GetRelativeLocation (Variables|Default|GetLocatorClimbDown)) _relativelocation)))
  ;[1 1 1] Set New Locations
  (Transformation|SetRelativeLocation (Variables|Default|GetBindingAreaTop) (LocalVariables|GetBindTarget) false false)
  (Transformation|SetRelativeLocation (Variables|Default|GetEndAreaClimbUp) (LocalVariables|GetEndTarget) false false)
  (Transformation|SetRelativeLocation (Variables|Default|GetLocatorClimbDown) (Math|Vector|MakeVector (.x (LocalVariables|GetLocTarget)) (.y (LocalVariables|GetLocTarget)) (+ (.z (LocalVariables|GetLocTarget)) 9.0)) false false))

(fn SetupMiddle
  (bind _bindingareamiddle (Variables|Default|GetBindingAreaMiddle))
  (bind _bindingareamiddle_2 (Variables|Default|GetBindingAreaMiddle))
  (bind _relativelocation (Variables|/Script/Engine.SceneComponent|GetRelativeLocation _bindingareamiddle))
  (bind _boxextent (Variables|/Script/Engine.BoxComponent|GetBoxExtent _bindingareamiddle_2))
  (LocalVariables|SetMid (* (Utilities|GetHeightValue) 0.5))
  (Transformation|SetRelativeLocation _bindingareamiddle (Math|Vector|MakeVector (.x _relativelocation) (.y _relativelocation) (LocalVariables|GetMid)) false false)
  (Components|Box|SetBoxExtent _bindingareamiddle_2 (Math|Vector|MakeVector (.x _boxextent) (.y _boxextent) (LocalVariables|GetMid)) true))

(fn QueryComponents
  (for _array_element (Actor|GetComponentsByClass (Variables|Default|GetLadder) "/Script/Engine.SceneComponent")
    (switch string (Utilities|GetObjectName _array_element)
      (:EndAreaClimbUp
        (bind _asbox_collision (Utilities|Casting|CastToBoxComponent _array_element))
        (Variables|Default|SetEndAreaClimbUp _asbox_collision))
      (:BindingAreaTop
        (bind _asbox_collision_2 (Utilities|Casting|CastToBoxComponent _array_element))
        (Variables|Default|SetBindingAreaTop _asbox_collision_2))
      (:BindingAreaMiddle
        (bind _asbox_collision_3 (Utilities|Casting|CastToBoxComponent _array_element))
        (Variables|Default|SetBindingAreaMiddle _asbox_collision_3))
      (:LocatorClimbDown
        (Variables|Default|SetLocatorClimbDown _array_element))
      (:SM_SpLadder01a_st05a1
        (bind _asstatic_mesh_component (Utilities|Casting|CastToStaticMeshComponent _array_element))
        (Variables|Default|SetBottomMesh _asstatic_mesh_component))
      (:SM_SpLadder01b_st05a1
        (bind _asstatic_mesh_component_2 (Utilities|Casting|CastToStaticMeshComponent _array_element))
        (Variables|Default|SetTopMesh _asstatic_mesh_component_2))
      (:LadderNavLink
        (bind _aschild_actor_component (Utilities|Casting|CastToChildActorComponent _array_element))
        (Variables|Default|SetLadderNavLink _aschild_actor_component)))))

(fn AdjustHeight
  (if (Variables|Ladder|GetKeepAligned)
    (Variables|Ladder|SetHeight (* (.ReturnValue (Math|Float|Division(WholeandRemainder) (Variables|Ladder|GetHeight) 5e+01)) 5e+01))))